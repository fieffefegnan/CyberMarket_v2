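; Graffiti decal actor for environment dressing, configured entirely in the Construction Script with no runtime logic.
; X and Y snap to quarter steps from 0 to 0.75, apparently selecting a cell in a 4x4 texture atlas.
; The Cube component hosts a dynamic material instance that receives these offsets plus wear, opacity and color values.
; That material is then assigned to the Decal component.
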(fn `UserConstructionScript`
  (bind _cube (`self.Cube`))
  (bind _cube_2 (`self.Cube`))
  (bind _cube_3 (`self.Cube`))
  (bind _cube_4 (`self.Cube`))
  (`MeshComponent.SetScalarParameterValueOnMaterials` _cube_2 "X" (`self.X`))
  (`MeshComponent.SetScalarParameterValueOnMaterials` _cube_2 "Y" (`self.Y`))
  (bind _returnvalue (`PrimitiveComponent.CreateDynamicMaterialInstance` (`self.Cube`) 0 null "None"))
  (bind _returnvalue_2 (`MaterialInstanceDynamic.K2_GetScalarParameterValue` _returnvalue "X"))
  (if (< _returnvalue_2 0.25)
    (`MeshComponent.SetScalarParameterValueOnMaterials` _cube "X" 0.0)
    (set `self.X` 0.0)
    (elif (< _returnvalue_2 0.5)
      (`MeshComponent.SetScalarParameterValueOnMaterials` _cube "X" 0.25)
      (set `self.X` 0.25)
      (elif (< _returnvalue_2 0.75)
        (`MeshComponent.SetScalarParameterValueOnMaterials` _cube "X" 0.5)
        (set `self.X` 0.5)
        (elif (< _returnvalue_2 1.0)
          (`MeshComponent.SetScalarParameterValueOnMaterials` _cube "X" 0.75)
          (set `self.X` 0.75)
          (else
            (set `self.X` 0.75)
            (`MeshComponent.SetScalarParameterValueOnMaterials` _cube "X" 0.75))))))
  (bind _returnvalue_3 (`MaterialInstanceDynamic.K2_GetScalarParameterValue` _returnvalue "Y"))
  (if (< _returnvalue_3 0.25)
    (`MeshComponent.SetScalarParameterValueOnMaterials` _cube_3 "Y" 0.0)
    (set `self.Y` 0.0)
    (elif (< _returnvalue_3 0.5)
      (`MeshComponent.SetScalarParameterValueOnMaterials` _cube_3 "Y" 0.25)
      (set `self.Y` 0.25)
      (elif (< _returnvalue_3 0.75)
        (`MeshComponent.SetScalarParameterValueOnMaterials` _cube_3 "Y" 0.5)
        (set `self.Y` 0.5)
        (elif (< _returnvalue_3 1.0)
          (`MeshComponent.SetScalarParameterValueOnMaterials` _cube_3 "Y" 0.75)
          (set `self.Y` 0.75)
          (else
            (`MeshComponent.SetScalarParameterValueOnMaterials` _cube_3 "Y" 0.75)
            (set `self.Y` 0.75))))))
  (`MeshComponent.SetScalarParameterValueOnMaterials` _cube_4 "WearValue" (`self.WearValue`))
  (`MeshComponent.SetScalarParameterValueOnMaterials` _cube_4 "Opacity" (`self.Opacity`))
  (`MeshComponent.SetScalarParameterValueOnMaterials` _cube_4 "ColorValue" (`self.ColorValue`))
  (`DecalComponent.SetDecalMaterial` (`self.Decal`) (`PrimitiveComponent.GetMaterial` _cube_4 0)))